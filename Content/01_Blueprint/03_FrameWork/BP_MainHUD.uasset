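; BP_MainHUD is the HUD Blueprint that manages the main, setting and inventory UI widgets.
; On BeginPlay it creates the main UI for player controller 0, adds it to the viewport and stores the reference.
; SetSettingUI and SetInventoryUI lazily create their widget on first use, then reuse the stored instance by making it visible, giving it focus in both cases.
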(event Custom|SetSettingUI
  (Utilities|IsValid (Variables|Default|GetSettingUI)
    (:Is%20Valid
      (Widget|SetVisibility (Variables|Default|GetSettingUI) "Visible")
      (Widget|SetFocus (Variables|Default|GetSettingUI)))
    (:Is%20Not%20Valid
      (bind _returnvalue (UserInterface|CreateWidget "/Game/01_Blueprint/04_UI/SettingUI.SettingUI_C"))
      (bind _output_get (Variables|Default|SetSettingUI _returnvalue))
      (UserInterface|Viewport|AddtoViewport _output_get 0)
      (Widget|SetFocus (Variables|Default|GetSettingUI)))))

(event Custom|SetInventoryUI
  (Utilities|IsValid (Variables|Default|GetInventoryUI)
    (:Is%20Valid
      (Widget|SetVisibility (Variables|Default|GetInventoryUI) "Visible")
      (Widget|SetFocus (Variables|Default|GetInventoryUI)))
    (:Is%20Not%20Valid
      (bind _returnvalue (UserInterface|CreateWidget "/Game/01_Blueprint/04_UI/InventoryUI.InventoryUI_C"))
      (bind _output_get (Variables|Default|SetInventoryUI _returnvalue))
      (UserInterface|Viewport|AddtoViewport _output_get 0)
      (Widget|SetFocus (Variables|Default|GetInventoryUI)))))

(event EventBeginPlay
  (bind _returnvalue (UserInterface|CreateWidget "/Game/01_Blueprint/04_UI/MainUI.MainUI_C" (Game|GetPlayerController 0)))
  (UserInterface|Viewport|AddtoViewport _returnvalue 0)
  (Variables|Default|SetMainUI _returnvalue))

(event Collision|EventActorBeginOverlap
  (params (OtherActor :type Actor%20Object%20Reference)))

(event EventTick
  (params (DeltaSeconds :type Float%20%28single-precision%29)))

(fn ConstructionScript)