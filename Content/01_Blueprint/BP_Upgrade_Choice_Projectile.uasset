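; An actor whose mesh shuttles between its start position and a target component's position while firing a BP_Projectile every second, offset along the actor's forward vector.
; Tick advances the mesh at Speed, swapping start and target once the traveled distance covers the path length.
; IsWaitCube selects WaitMove, which pauses two seconds at each end, or DontStopMove, which reverses immediately.
; Firing runs on its own accumulated timer, so it continues during pauses.
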(event EventBeginPlay
  (Variables|Default|SetStartLocation (Variables|/Script/Engine.SceneComponent|GetRelativeLocation (Variables|Default|GetStaticMesh)))
  (Variables|Default|SetTargetLocation (Variables|/Script/Engine.SceneComponent|GetRelativeLocation (Variables|Default|GetTargetCompoment))))

(event Collision|EventActorBeginOverlap
  (params (OtherActor :type Actor%20Object%20Reference)))

(event EventTick
  (params (DeltaSeconds :type Float%20%28single-precision%29))
  (bind _staticmesh (Variables|Default|GetStaticMesh))
  (bind _returnvalue (Transformation|GetWorldTransform _staticmesh))
  (Utilities|FlowControl|Sequence
    (:then_0
      (if (Variables|Default|GetIsWaitCube)
        (CallFunction|WaitMove DeltaSeconds)
        (else
          (CallFunction|DontStopMove DeltaSeconds))))
    (:then_1
      (bind _output_get (Variables|Default|SetProjectileAcctime (+ (Variables|Default|GetProjectileAcctime) DeltaSeconds)))
      (if (>= _output_get 1.0)
        (Game|SpawnActorfromClass "/Game/01_Blueprint/01_Character/BP_Projectile.BP_Projectile_C" (Math|Transform|MakeTransform (+ (.location _returnvalue) (* (Transformation|GetActorForwardVector) 5e+01)) (.rotation _returnvalue) (.scale _returnvalue)) "Undefined" "MultiplyWithRoot" 0 0)
        (Variables|Default|SetProjectileAcctime 0.0)))))

(fn ConstructionScript)

(fn MoveUpdate
  (params (DeltaTime :type Float%20%28double-precision%29))
  ;[1 1 1] 이동
  (Transformation|SetRelativeLocation (Variables|Default|GetStaticMesh) (+ (Variables|/Script/Engine.SceneComponent|GetRelativeLocation (Variables|Default|GetStaticMesh)) (* (Math|Vector|Normalize (- (Variables|Default|GetTargetLocation) (Variables|Default|GetStartLocation))) (* (Variables|Default|GetSpeed) DeltaTime))) false false))

(fn LengthCheck
  ;[1 1 1] 가야 할 거리
  (Variables|Default|SetLength (Math|Vector|VectorLength (- (Variables|Default|GetTargetLocation) (Variables|Default|GetStartLocation))))
  ;[1 1 1] 가고 있는 거리
  (Variables|Default|SetTravelled (Math|Vector|VectorLength (- (Variables|/Script/Engine.SceneComponent|GetRelativeLocation (Variables|Default|GetStaticMesh)) (Variables|Default|GetStartLocation)))))

(fn Shufle
  (bind _travelled (Variables|Default|GetTravelled))
  (bind _length (Variables|Default|GetLength))
  (bind _returnvalue (>= _travelled _length))
  ;[1 1 1] 위치를 셔플로 바꾸기
  (if _returnvalue
    (Variables|Default|SetTempLocation (Variables|Default|GetStartLocation))
    (Variables|Default|SetStartLocation (Variables|Default|GetTargetLocation))
    (Variables|Default|SetTargetLocation (Variables|Default|GetTempLocation))
    (return _returnvalue)
    (else
      (return false))))

(fn WaitTimeCheck
  (params (DeltaTime :type Float%20%28double-precision%29))
  (bind _output_get (Variables|Default|SetAcctime (+ (Variables|Default|GetAcctime) DeltaTime)))
  (if (>= _output_get 2.0)
    (Variables|Default|SetIsWait false)
    (Variables|Default|SetAcctime 0.0)))

(fn WaitMove
  (params (DeltaTime :type Float%20%28double-precision%29))
  (if (Variables|Default|GetIsWait)
    (CallFunction|WaitTimeCheck DeltaTime)
    (else
      (CallFunction|LengthCheck)
      (bind _ischange (CallFunction|Shufle))
      (Variables|Default|SetIsWait _ischange)
      (CallFunction|MoveUpdate DeltaTime))))

(fn DontStopMove
  (params (DeltaTime :type Float%20%28double-precision%29))
  (CallFunction|LengthCheck)
  (CallFunction|Shufle)
  (CallFunction|MoveUpdate DeltaTime))