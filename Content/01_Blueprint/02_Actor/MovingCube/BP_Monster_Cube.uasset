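; BP_Monster_Cube is a cube actor that moves back and forth on a timer.
; Tick accumulates delta time in AccDistance and moves the actor along normalized Dir at Speed without sweep.
; After more than three seconds it resets the timer and multiplies Dir by a negative Y-only vector, reversing Y and zeroing X and Z.
; A Stop flag is true while moving and is set false and printed at each reversal.
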(event EventBeginPlay)

(event Collision|EventActorBeginOverlap
  (params (OtherActor :type Actor%20Object%20Reference)))

(event EventTick
  (params (DeltaSeconds :type Float%20%28single-precision%29))
  (Utilities|FlowControl|Sequence
    (:then_0
      ;[1 1 1] 누적 1초 계산
      (Variables|Default|SetAccDistance (+ (Variables|Default|GetAccDistance) DeltaSeconds)))
    (:then_1
      ;[1 1 1] 액터 이동 시간 제한
      (if (> (Variables|Default|GetAccDistance) 3.0)
        ;[1 1 1] 3초 -> 0초로 초기화, 방향 벡터 반대로 바꾸기
        (Variables|Default|SetAccDistance 0.0)
        (Variables|Default|SetDir (* (Variables|Default|GetDir) "0.000000,-1.000000,0.000000"))
        (bind _output_get (Variables|Default|SetStop false))
        (Development|PrintString (Utilities|String|ToString(Boolean) _output_get))
        (else
          ;[1 1 1] 정해진 시간만큼 올라갔다 내려가기 반복
          (Transformation|SetActorLocation (+ (Transformation|GetActorLocation) (* (* (Math|Vector|Normalize (Variables|Default|GetDir)) (Variables|Default|GetSpeed)) DeltaSeconds)) false false)
          (Variables|Default|SetStop true))))))

(fn ConstructionScript)